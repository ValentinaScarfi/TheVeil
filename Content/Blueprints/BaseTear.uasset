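; Base tear actor that the player sews by touching all its eyelets while carrying a matching absorbed colour.
; SetTearColour tints the dynamic material and spawns Eyelet actors at tagged placeholder meshes.
; When VeilCharacter's overlap ends, guarded by a delayed flag against plane switching, missed eyelets cause damage and reset combo.
; Completed tears raise combo and score, with colour mismatches earning less and filling an error bar that deals damage when full.
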(event OnComponentBeginOverlap(TearCollider)
  (params (OverlappedComponent :type Primitive%20Component%20Object%20Reference) (OtherActor :type Actor%20Object%20Reference) (OtherComp :type Primitive%20Component%20Object%20Reference) (OtherBodyIndex :type Integer) (bFromSweep :type Boolean) (SweepResult :type Hit%20Result%20Structure%20%28by%20ref%29))
  ;[1 1 1] Used to be sure that switching planes won't make the overlap between tear and player end instantly
  (Utilities|Casting|CastToVeilCharacter OtherActor)
  (Utilities|FlowControl|Delay 0.3)
  (Variables|Default|SetisStillOverlapping true))

(event OnComponentEndOverlap(TearCollider)
  (params (OverlappedComponent :type Primitive%20Component%20Object%20Reference) (OtherActor :type Actor%20Object%20Reference) (OtherComp :type Primitive%20Component%20Object%20Reference) (OtherBodyIndex :type Integer))
  (bind _tearmaterialcolour (Variables|Default|GetTearMaterialColour))
  (bind _alleyeletstouched (Variables|Default|GetallEyeletsTouched))
  (bind _asveil_character (Utilities|Casting|CastToVeilCharacter OtherActor))
  (Variables|Default|SetThisCharacter _asveil_character)
  (if (Variables|Default|GetisStillOverlapping)
    (for _array_element (Variables|Default|GetEyelets) ; Checking if player has touched all eyelets of tear
      (Utilities|Array|Add (Variables|Default|GetallEyeletsTouched) (Variables|/Game/Blueprints/Eyelet.Eyelet_C|GethasBeenOverlapped _array_element)) ; Adding overlapped flags of eyelets to
    )
    (if (Utilities|Array|ContainsItem _alleyeletstouched false)
      (Utilities|Array|Clear _alleyeletstouched)
      (Utilities|FlowControl|DoOnce false ; Taking damage once if player misses eyelet(s)
        (:Completed
          (Default|TakeDamage (Variables|Default|GetThisCharacter))
          (Variables|/Game/Blueprints/VeilCharacter.VeilCharacter_C|SetCombo (Variables|Default|GetThisCharacter) 0)
          (Rendering|Material|SetVectorParameterValue (Variables|/Game/Blueprints/VeilCharacter.VeilCharacter_C|GetAbsorbedColourMat (Variables|Default|GetThisCharacter)) "AbsorbedColour" "(R=0.000000,G=0.000000,B=0.000000,A=1.000000)" :!class /Script/Engine.MaterialInstanceDynamic :!label _label) ; Resetting colour indicator to black after tear has passed
          (Utilities|Array|Clear (Variables|/Game/Blueprints/VeilCharacter.VeilCharacter_C|GetCurrentColoursAbsorbed (Variables|Default|GetThisCharacter)))))
      (else
        (bind _currentcolourofcharacter (Default|GetCurrentColourAbsorbed (Variables|Default|GetThisCharacter))) ; Getting current colour of indicator (only RGB values to make a new vector)
        (Variables|Default|SetCharacterColourVector (Math|Vector|MakeVector (.r _currentcolourofcharacter) (.g _currentcolourofcharacter) (.b _currentcolourofcharacter)))
        (bind _output_get (Variables|Default|SetTearColourVector (Math|Vector|MakeVector (.r _tearmaterialcolour) (.g _tearmaterialcolour) (.b _tearmaterialcolour))))
        (Utilities|FlowControl|DoOnce false
          (:Completed
            (Math|Integer|IncrementInt (Variables|/Game/Blueprints/VeilCharacter.VeilCharacter_C|GetCombo (Variables|Default|GetThisCharacter))
              (:%20%20
                (if (Math|Vector|Equal(Vector) _output_get (Variables|Default|GetCharacterColourVector) 0.0001) ; If they match, nothing happens (SCORE - to be done)
                  (Default|AddScore (Variables|Default|GetThisCharacter) 20 (Utilities|Array|Length (Variables|Default|GetEyelets)) (Variables|/Game/Blueprints/VeilCharacter.VeilCharacter_C|GetCombo (Variables|Default|GetThisCharacter)))
                  (goto _label)
                  (else
                    (Utilities|FlowControl|DoOnce false ; If they don't match, the Error Tolerance bar increases by 25%
                      (:Completed
                        (Default|AddScore (Variables|Default|GetThisCharacter) 10 (Utilities|Array|Length (Variables|Default|GetEyelets)) (Variables|/Game/Blueprints/VeilCharacter.VeilCharacter_C|GetCombo (Variables|Default|GetThisCharacter)))
                        (bind _output_get_2 (Variables|/Game/Blueprints/VeilCharacter.VeilCharacter_C|SetErrorProgression (Variables|Default|GetThisCharacter) (+ (Variables|/Game/Blueprints/VeilCharacter.VeilCharacter_C|GetErrorProgression (Variables|Default|GetThisCharacter)) 0.25)))
                        (if (== _output_get_2 1.0) ; If error tolerance reaches 100%, player takes damage and absorbed colour is reset to black
                          (Default|TakeDamage (Variables|Default|GetThisCharacter))
                          (Rendering|Material|SetVectorParameterValue (Variables|/Game/Blueprints/VeilCharacter.VeilCharacter_C|GetAbsorbedColourMat (Variables|Default|GetThisCharacter)) "AbsorbedColour" "(R=0.000000,G=0.000000,B=0.000000,A=1.000000)" :!class /Script/Engine.MaterialInstanceDynamic) ; Resetting colour indicator to black after tear has passed
                          (Utilities|Array|Clear (Variables|/Game/Blueprints/VeilCharacter.VeilCharacter_C|GetCurrentColoursAbsorbed (Variables|Default|GetThisCharacter)))
                          (Utilities|FlowControl|Delay 0.5) ; Adding some delay to show bar getting full before emptying it again
                          (Variables|/Game/Blueprints/VeilCharacter.VeilCharacter_C|SetErrorProgression (Variables|Default|GetThisCharacter) 0.0)
                          (else
                            (goto _label)))))))))))))))

(event EventBeginPlay)

(event Collision|EventActorBeginOverlap
  (params (OtherActor :type Actor%20Object%20Reference)))

(fn ConstructionScript
  (bind _returnvalue (Rendering|Material|CreateDynamicMaterialInstance (Variables|Default|GetPlane) 0 (Rendering|Material|GetMaterial (Variables|Default|GetPlane) 0) :!class /Script/Engine.PrimitiveComponent)) ; Creating dynamic material for tear to change colour
  (Variables|Default|SetTearMaterial _returnvalue))

(fn SetTearColour
  (switch int (Variables|Default|GetTearColour) ; Setting material colour according to int
    (:Default
      (Variables|Default|SetTearMaterialColour "(R=0.000000,G=0.972549,B=1.000000,A=1.000000)" :!label _label))
    (:0
      (Variables|Default|SetTearMaterialColour "(R=0.003922,G=1.000000,B=0.000000,A=1.000000)"))
    (:1
      (Variables|Default|SetTearMaterialColour "(R=1.000000,G=0.321569,B=0.000000,A=1.000000)"))
    (:2
      (Variables|Default|SetTearMaterialColour "(R=0.592157,G=0.000000,B=1.000000,A=1.000000)"))
    (:3
      (Variables|Default|SetTearMaterialColour "(R=1.000000,G=0.184314,B=0.388533,A=1.000000)"))
    (:4
      (goto _label)))
  (Rendering|Material|SetVectorParameterValue (Variables|Default|GetTearMaterial) "TearColour" (Variables|Default|GetTearMaterialColour) :!class /Script/Engine.MaterialInstanceDynamic)
  (bind _output_get (Variables|Default|SetEyeletsPlaceHolders (Actor|GetComponentsbyTag self "/Script/Engine.StaticMeshComponent" "Eyelet")))
  (for _array_element _output_get ; Foreach placeholder
    (bind _returnvalue (Game|SpawnActorfromClass "/Game/Blueprints/Eyelet.Eyelet_C" (Transformation|GetWorldTransform _array_element) "Undefined" 0 0)) ; Spawn eyelet actors on sphere placeholders
    (Variables|/Game/Blueprints/Eyelet.Eyelet_C|SetEyeletValidationColour _returnvalue (Variables|Default|GetTearMaterialColour)) ; Setting eyelet validation colour to tear colour
    (Utilities|Array|Add (Variables|Default|GetEyelets) _returnvalue) ; Adding nw eyelet spawned to array of tear eyelets
  ))