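; EnemySpawner Blueprint that places a GenericEnemy on its associated tile (ThisTile) each time Spawn is called.
; Spawn picks a random X around the tile's EnemySpawnOrigin, creates the enemy and sets itself as its MySpawner.
; It then sets the enemy's height from collider extent and floor mesh bounds, negated for upside-down enemies, and adds it to the tile's Enemies list.
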(event EventBeginPlay)

(event Collision|EventActorBeginOverlap
  (params (OtherActor :type Actor%20Object%20Reference)))

(event EventTick
  (params (DeltaSeconds :type Float%20%28single-precision%29)))

(fn ConstructionScript)

(fn Spawn
  (bind _randomxpos (CallFunction|DetermineXRandomPosition))
  (bind _returnvalue (Game|SpawnActorfromClass "/Game/Blueprints/GenericEnemy.GenericEnemy_C" (Math|Transform|MakeTransform (Math|Vector|MakeVector (Math|Conversions|ToFloat(Integer) _randomxpos) 0.0 0.0) "0, 0, 0" "1,1,1") "Undefined" 0 0))
  (Variables|/Game/Blueprints/GenericEnemy.GenericEnemy_C|SetMySpawner _returnvalue self)
  (bind _movedenemy (CallFunction|DetermineZPositionandOrientation _returnvalue))
  (Utilities|Array|Add (Variables|/Game/Blueprints/Tile.Tile_C|GetEnemies (Variables|Default|GetThisTile)) _movedenemy))

(fn DetermineZPositionandOrientation
  (params (Enemy :type Generic%20Enemy%20Object%20Reference))
  (bind _thistile (Variables|Default|GetThisTile))
  (bind _enemycollider (Variables|/Game/Blueprints/GenericEnemy.GenericEnemy_C|GetEnemyCollider Enemy))
  (bind _floor (Variables|/Game/Blueprints/Tile.Tile_C|GetFloor _thistile))
  (bind _boxextent (Variables|/Script/Engine.BoxComponent|GetBoxExtent _enemycollider))
  (bind _relativelocation (Variables|/Script/Engine.SceneComponent|GetRelativeLocation _enemycollider))
  (bind _staticmesh (Variables|/Script/Engine.StaticMeshComponent|GetStaticMesh _floor))
  (bind _returnvalue (StaticMesh|GetBoundingBox _staticmesh))
  (bind _returnvalue_2 (+ (.z _boxextent) (.z (.max _returnvalue))))
  (if (Variables|/Game/Blueprints/GenericEnemy.GenericEnemy_C|GetisUpsideDown Enemy)
    (Transformation|SetActorRelativeLocation Enemy (Math|Vector|MakeVector (.x _relativelocation) (.y _relativelocation) (* _returnvalue_2 -1.0)))
    (else
      (Transformation|SetActorRelativeLocation Enemy (Math|Vector|MakeVector (.x _relativelocation) (.y _relativelocation) _returnvalue_2))))
  (return Enemy))

(fn DetermineXRandomPosition
  (return (+ (Math|Float|Truncate (.x (Transformation|GetWorldLocation (Variables|/Game/Blueprints/Tile.Tile_C|GetEnemySpawnOrigin (Variables|Default|GetThisTile))))) (Math|Random|RandomIntegerinRange -2400 2400))))