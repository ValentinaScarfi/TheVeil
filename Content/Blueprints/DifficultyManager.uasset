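; Difficulty manager actor that steps the game through five levels as the VeilCharacter sews tears.
; It registers itself with the player on BeginPlay; CheckIfToNextLevel compares TearsSewn to the level's threshold, then increments the level and notifies the HUD.
; Each level resets the count and sets the threshold, TearSpawner pool, player speed and TileSpawner enemy settings.
; The camera is placed directly at level one, then eased by per-level timelines.
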(event Custom|SmoothCamera
  (bind _thischaracter (Variables|Default|GetThisCharacter))
  (bind _camerachar (Variables|/Game/Blueprints/VeilCharacter.VeilCharacter_C|GetCameraChar _thischaracter))
  (switch int (Variables|Default|GetDifficultyLevel)
    (:2
      (bind (_direction _cameraposition _camerarotation) (Timeline|CameraAnimation1 Play)
        (:Update
          (Transformation|SetRelativeLocationAndRotation _camerachar (Math|Vector|MakeVector 0.0 _cameraposition 5e+01) (Math|Rotator|MakeRotator _camerarotation 0.0 0.0) false false))))
    (:3
      (bind (_direction_2 _cameraposition_2 _camerarotation_2) (Timeline|CameraAnimation2 Play)
        (:Update
          (Transformation|SetRelativeLocationAndRotation _camerachar (Math|Vector|MakeVector 0.0 _cameraposition_2 5e+01) (Math|Rotator|MakeRotator _camerarotation_2 0.0 0.0) false false))))
    (:4
      (bind (_direction_3 _cameraposition_3 _camerarotation_3) (Timeline|CameraAnimation3 Play)
        (:Update
          (Transformation|SetRelativeLocationAndRotation _camerachar (Math|Vector|MakeVector 0.0 _cameraposition_3 5e+01) (Math|Rotator|MakeRotator _camerarotation_3 0.0 0.0) false false))))
    (:5
      (bind _camerarotation_4 (Timeline|CameraAnimation4 Play)
        (:Update
          (Transformation|SetRelativeLocationAndRotation _camerachar (Math|Vector|MakeVector 0.0 0.0 5e+01) (Math|Rotator|MakeRotator _camerarotation_4 0.0 0.0) false false))))))

(event EventBeginPlay
  (bind _asveil_character (Utilities|Casting|CastToVeilCharacter (Game|GetPlayerCharacter 0)))
  (bind _output_get (Variables|Default|SetThisCharacter _asveil_character))
  (Variables|/Game/Blueprints/VeilCharacter.VeilCharacter_C|SetDifficultyManagerRef _output_get self)
  (CallFunction|SetNewDifficultyValues))

(event Collision|EventActorBeginOverlap
  (params (OtherActor :type Actor%20Object%20Reference)))

(event EventTick
  (params (DeltaSeconds :type Float%20%28single-precision%29)))

(fn ConstructionScript)

(fn SetThresholdtoNextLevel
  (switch int (Variables|Default|GetDifficultyLevel)
    (:1
      (Variables|Default|SetTearThreshold 1))
    (:2
      (Variables|Default|SetTearThreshold 4))
    (:3
      (Variables|Default|SetTearThreshold 6))
    (:4
      (Variables|Default|SetTearThreshold 5))
    (:5
      (Variables|Default|SetTearThreshold 4))))

(fn SetTearPool
  (bind _tearspawner (Variables|Default|GetTearSpawner))
  (bind _tearspawner_2 (Variables|Default|GetTearSpawner))
  (bind _tear6classes (Variables|/Game/Blueprints/TearSpawner.TearSpawner_C|GetTear6Classes _tearspawner_2))
  (bind _currenttearspool (Variables|/Game/Blueprints/TearSpawner.TearSpawner_C|GetCurrentTearsPool _tearspawner))
  (Utilities|Array|Clear _currenttearspool)
  (switch int (Variables|Default|GetDifficultyLevel)
    (:1
      (Utilities|Array|AppendArray _currenttearspool (Variables|/Game/Blueprints/TearSpawner.TearSpawner_C|GetTear3Classes _tearspawner)))
    (:2
      (Utilities|Array|AppendArray _currenttearspool (Variables|/Game/Blueprints/TearSpawner.TearSpawner_C|GetTear4Classes _tearspawner)))
    (:3
      (Utilities|Array|AppendArray _currenttearspool (Variables|/Game/Blueprints/TearSpawner.TearSpawner_C|GetTear5Classes _tearspawner_2))
      (Utilities|Array|AppendArray _currenttearspool _tear6classes))
    (:4
      (Utilities|Array|AppendArray _currenttearspool _tear6classes)
      (Utilities|Array|AppendArray _currenttearspool (Variables|/Game/Blueprints/TearSpawner.TearSpawner_C|GetTear7Classes _tearspawner_2)))
    (:5
      (Utilities|Array|AppendArray _currenttearspool (Variables|/Game/Blueprints/TearSpawner.TearSpawner_C|GetTear8Classes _tearspawner_2)))))

(fn CheckiftoNextLevel
  (if (== (Variables|/Game/Blueprints/VeilCharacter.VeilCharacter_C|GetTearsSewn (Variables|Default|GetThisCharacter)) (Variables|Default|GetTearThreshold))
    (if (< (Variables|Default|GetDifficultyLevel) 5)
      (Math|Integer|IncrementInt (Variables|Default|GetDifficultyLevel)
        (:%20%20
          (Default|SeeDifficultyChange (Variables|/Game/Blueprints/VeilCharacter.VeilCharacter_C|GetHUD (Variables|Default|GetThisCharacter)))
          (CallFunction|SetNewDifficultyValues))))))

(fn SetNewDifficultyValues
  (Variables|/Game/Blueprints/VeilCharacter.VeilCharacter_C|SetTearsSewn (Variables|Default|GetThisCharacter) 0)
  (CallFunction|SetThresholdtoNextLevel)
  (CallFunction|SetTearPool)
  (CallFunction|SetPlayerSpeed)
  (CallFunction|SetNumberOfEnemies)
  (CallFunction|SetMaxTileswithEnemies)
  (CallFunction|SetPercentageOfAppropriateEnemies)
  (CallFunction|SetCameraPosandRot))

(fn SetPlayerSpeed
  (bind _thischaracter (Variables|Default|GetThisCharacter))
  (switch int (Variables|Default|GetDifficultyLevel)
    (:1
      (Variables|/Game/Blueprints/VeilCharacter.VeilCharacter_C|SetSpeed _thischaracter 1.5e+03))
    (:2
      (Variables|/Game/Blueprints/VeilCharacter.VeilCharacter_C|SetSpeed _thischaracter 1.75e+03))
    (:3
      (Variables|/Game/Blueprints/VeilCharacter.VeilCharacter_C|SetSpeed _thischaracter 2e+03))
    (:4
      (Variables|/Game/Blueprints/VeilCharacter.VeilCharacter_C|SetSpeed _thischaracter 2.25e+03))
    (:5
      (Variables|/Game/Blueprints/VeilCharacter.VeilCharacter_C|SetSpeed _thischaracter 2.5e+03))))

(fn SetNumberOfEnemies
  (bind _tilespawner (Variables|Default|GetTileSpawner))
  (switch int (Variables|Default|GetDifficultyLevel)
    (:1
      (Variables|/Game/Blueprints/TileSpawner.TileSpawner_C|SetNumberOfEnemiesPerTile _tilespawner 2)
      (Variables|/Game/Blueprints/TileSpawner.TileSpawner_C|SetMinDistanceEnemies _tilespawner 1500))
    (:2
      (Variables|/Game/Blueprints/TileSpawner.TileSpawner_C|SetNumberOfEnemiesPerTile _tilespawner 3)
      (Variables|/Game/Blueprints/TileSpawner.TileSpawner_C|SetMinDistanceEnemies _tilespawner 1000))
    (:3
      (Variables|/Game/Blueprints/TileSpawner.TileSpawner_C|SetNumberOfEnemiesPerTile _tilespawner 3)
      (Variables|/Game/Blueprints/TileSpawner.TileSpawner_C|SetMinDistanceEnemies _tilespawner 1000))
    (:4
      (Variables|/Game/Blueprints/TileSpawner.TileSpawner_C|SetNumberOfEnemiesPerTile _tilespawner 4)
      (Variables|/Game/Blueprints/TileSpawner.TileSpawner_C|SetMinDistanceEnemies _tilespawner 750))
    (:5
      (Variables|/Game/Blueprints/TileSpawner.TileSpawner_C|SetNumberOfEnemiesPerTile _tilespawner 5)
      (Variables|/Game/Blueprints/TileSpawner.TileSpawner_C|SetMinDistanceEnemies _tilespawner 600))))

(fn SetMaxTileswithEnemies
  (bind _tilespawner (Variables|Default|GetTileSpawner))
  (switch int (Variables|Default|GetDifficultyLevel)
    (:1
      (Variables|/Game/Blueprints/TileSpawner.TileSpawner_C|SetMaxTilesWithEnemies _tilespawner 6))
    (:2
      (Variables|/Game/Blueprints/TileSpawner.TileSpawner_C|SetMaxTilesWithEnemies _tilespawner 5))
    (:3
      (Variables|/Game/Blueprints/TileSpawner.TileSpawner_C|SetMaxTilesWithEnemies _tilespawner 5))
    (:4
      (Variables|/Game/Blueprints/TileSpawner.TileSpawner_C|SetMaxTilesWithEnemies _tilespawner 4))
    (:5
      (Variables|/Game/Blueprints/TileSpawner.TileSpawner_C|SetMaxTilesWithEnemies _tilespawner 3))))

(fn SetPercentageOfAppropriateEnemies
  (bind _tilespawner (Variables|Default|GetTileSpawner))
  (switch int (Variables|Default|GetDifficultyLevel)
    (:1
      (Variables|/Game/Blueprints/TileSpawner.TileSpawner_C|SetPercentageOfAppropriateEnemies _tilespawner 35.0))
    (:2
      (Variables|/Game/Blueprints/TileSpawner.TileSpawner_C|SetPercentageOfAppropriateEnemies _tilespawner 3e+01))
    (:3
      (Variables|/Game/Blueprints/TileSpawner.TileSpawner_C|SetPercentageOfAppropriateEnemies _tilespawner 25.0))
    (:4
      (Variables|/Game/Blueprints/TileSpawner.TileSpawner_C|SetPercentageOfAppropriateEnemies _tilespawner 2e+01))
    (:5
      (Variables|/Game/Blueprints/TileSpawner.TileSpawner_C|SetPercentageOfAppropriateEnemies _tilespawner 2e+01))))

(fn SetCameraPosandRot
  (switch int (Variables|Default|GetDifficultyLevel)
    (:1
      (Transformation|SetRelativeLocationAndRotation (Variables|/Game/Blueprints/VeilCharacter.VeilCharacter_C|GetCameraChar (Variables|Default|GetThisCharacter)) "0,600.000000,50.000000" "0, 0,10.000000" false false))
    (:2
      (CallFunction|SmoothCamera))
    (:3
      (CallFunction|SmoothCamera))
    (:4
      (CallFunction|SmoothCamera))
    (:5
      (CallFunction|SmoothCamera))))