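; Tile spawner that builds a chain of random Biome1 tiles, turning one into a tear tile after a set number of enemy tiles.
; Each new tile attaches at the newest tile's spawn point and drives spawner references for enemies, or a coloured tear plus pickup.
; A tile counter times tear-colour changes and HUD updates.
; Enemy colours come from a shuffled pool seeded with a percentage of the two colours that combine into the tear's colour.
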(event EventBeginPlay
  (Variables|Default|SetCurrentColourOfTear (Math|Random|RandomIntegerinRange 0 4)) ; Setting first random colour of tear
  (CallFunction|SpawnInitialTiles))

(event Collision|EventActorBeginOverlap
  (params (OtherActor :type Actor%20Object%20Reference)))

(event EventTick
  (params (DeltaSeconds :type Float%20%28single-precision%29)))

(fn ConstructionScript)

(fn SpawnTile
  (params (SpawnLocation :type Vector))
  (bind _returnvalue (Game|SpawnActorfromClass (Utilities|Select :Index (Math|Random|RandomIntegerinRange 0 1) :Option%200 "/Game/Blueprints/Biome1_Tile1.Biome1_Tile1_C" :Option%201 "/Game/Blueprints/Biome1_Tile2.Biome1_Tile2_C") (Math|Transform|MakeTransform SpawnLocation "0, 0, 0" "50.000000,2.000000,1.000000") "Undefined" 0 0))
  (bind _asbase_tile (Utilities|Casting|CastToBaseTile _returnvalue))
  (bind _output_get (Variables|Default|SetNewestTile _asbase_tile))
  (Variables|/Game/Blueprints/BaseTile.BaseTile_C|SetTileSpawner _output_get self)
  (bind _asveil_character (Utilities|Casting|CastToVeilCharacter (Game|GetPlayerCharacter 0)))
  (Variables|/Game/Blueprints/VeilCharacter.VeilCharacter_C|SetInitialTile _asveil_character (Variables|Default|GetNewestTile))
  (if (> (Variables|Default|GetCounterToTearTile) (Variables|Default|GetMaxTilesWithEnemies))
    (Variables|/Game/Blueprints/BaseTile.BaseTile_C|SetisTearTile (Variables|Default|GetNewestTile) true)
    (Variables|Default|SetCounterToTearTile 0) ; Resetting counter after tear
  ))

(fn SpawnTileatSpawnPoint
  (bind _tearspawnerref (Variables|Default|GetTearSpawnerRef))
  (bind _newesttile (Variables|Default|GetNewestTile))
  (bind _newesttile_2 (Variables|Default|GetNewestTile))
  (bind _enemyspawnerref (Variables|Default|GetEnemySpawnerRef))
  (bind _spawnpoint (Variables|/Game/Blueprints/BaseTile.BaseTile_C|GetSpawnPoint _newesttile_2))
  (bind _currenttear (Variables|/Game/Blueprints/TearSpawner.TearSpawner_C|GetCurrentTear _tearspawnerref))
  (bind _enemiespositions (Variables|/Game/Blueprints/EnemySpawner.EnemySpawner_C|GetEnemiesPositions _enemyspawnerref))
  (bind _returnvalue (Transformation|GetWorldLocation _spawnpoint))
  ;[1 1 1] Spawning a new tile at spawning point defined in Tile class
  (CallFunction|SpawnTile (Math|Vector|MakeVector (+ (.x (.BoxExtent (Collision|GetComponentBounds (Variables|/Game/Blueprints/BaseTile.BaseTile_C|GetFloor _newesttile_2)))) (.x _returnvalue)) (.y _returnvalue) (.z _returnvalue)))
  ;[1 1 1] Set next colour when counter of tiles reaches defined values
  (Math|Integer|IncrementInt (Variables|Default|GetCounterToTearTile)
    (:%20%20
      (if (== (Variables|Default|GetCounterToTearTile) 2)
        (bind _output_get (Variables|Default|SetNewColourOfTear (Math|Random|RandomIntegerinRange 0 4)))
        (if (== _output_get (Variables|Default|GetCurrentColourOfTear)) :!label _label
          (Variables|Default|SetNewColourOfTear (Math|Random|RandomIntegerinRange 0 4))
          (goto _label)
          (else
            (Variables|Default|SetCurrentColourOfTear (Variables|Default|GetNewColourOfTear)))))
      (if (== (Variables|Default|GetCounterToTearTile) 4)
        (bind _asveil_character (Utilities|Casting|CastToVeilCharacter (Game|GetPlayerCharacter 0)))
        (Default|UpdateNextColour (Variables|/Game/Blueprints/VeilCharacter.VeilCharacter_C|GetHUD _asveil_character) (Variables|Default|GetCurrentColourOfTear)) ; Update HUD with next colour
      )
      ;[1 1 1] Setting current tile of enemy spawner and spawn new enemy - function is called here to avoid enemies to first tile spawned in world. Spawn algorithm determines random positions of enemies, spawn functions spawns all he enemies at the determined positions
      (Variables|/Game/Blueprints/EnemySpawner.EnemySpawner_C|SetThisTile (Variables|Default|GetEnemySpawnerRef) _newesttile :!pinned true) ; When new tile is spawned, the current "ThisTile" in spawner is set to newest tile spawned, to allow new enemies to spawn on it
      (if (Variables|/Game/Blueprints/BaseTile.BaseTile_C|GetisTearTile _newesttile)
        ;[1 1 1] Spawn tear on tear tile and set its colour, based on current colour
        (Default|SpawnTear _tearspawnerref)
        (Variables|/Game/Blueprints/BaseTile.BaseTile_C|SetmyTear (Variables|Default|GetNewestTile) _currenttear)
        (Variables|/Game/Blueprints/BaseTear.BaseTear_C|SetTearColour _currenttear (Variables|Default|GetCurrentColourOfTear))
        (Default|SetTearColour _currenttear)
        (Default|SpawnPickup (Variables|Default|GetPickupSpawnerRef))
        (else
          (Variables|/Game/Blueprints/BaseTile.BaseTile_C|SetTileID (Variables|Default|GetNewestTile) (- (Variables|Default|GetCounterToTearTile) 1))
          (Default|SpawnAlgorithm _enemyspawnerref 3 1000) ; Spawn n enemies at x positions
          ;[1 1 1] Seeding correct colour of enemies
          (Variables|Default|SetNumberOfEnemiesPerTile (Utilities|Array|Length _enemiespositions))
          (if (== (Variables|Default|GetIndexOfArrayOfColours) 0)
            (CallFunction|SeedingArrayOfEnemyColours (Variables|Default|GetNumberOfEnemiesPerTile) (Variables|Default|GetCurrentColourOfTear)) ; Seeding enemies colours to be sure player has the chance to form the right combination
          )
          (for (_array_element _array_index) _enemiespositions
            (Default|Spawn (Variables|Default|GetEnemySpawnerRef) _array_element (Utilities|Array|Get(acopy) (Variables|Default|GetAllColours) (+ _array_index (* (Variables|Default|GetIndexOfArrayOfColours) (Variables|Default|GetNumberOfEnemiesPerTile))))))
          (Utilities|Array|Clear (Variables|/Game/Blueprints/EnemySpawner.EnemySpawner_C|GetEnemiesPositions (Variables|Default|GetEnemySpawnerRef))) ; Clear enemies positions to not overlap with new ones
          (if (== (Variables|/Game/Blueprints/BaseTile.BaseTile_C|GetTileID (Variables|Default|GetNewestTile)) (Variables|Default|GetMaxTilesWithEnemies))
            (Utilities|Array|Clear (Variables|Default|GetAllColours)) ; Array of colour is cleared as all the colours have been used
            (Variables|Default|SetIndexOfArrayOfColours 0)
            (else
              (bind _result (Math|Integer|IncrementInt (Variables|Default|GetIndexOfArrayOfColours)) ; Index of colours increases as last tile with enemies has not been reached yet
                (:%20%20
                  (Variables|Default|SetIndexOfArrayOfColours _result))))))))))

(fn SpawnInitialTiles
  ;[1 1 1] Tile Spawner - if first tile doesn't exist, spawns it at player location, followed by another tile at the spawn point
  (for _index (range 0 2)
    (Utilities|IsValid (Variables|Default|GetNewestTile)
      (:Is%20Valid
        (CallFunction|SpawnTileatSpawnPoint))
      (:Is%20Not%20Valid
        (CallFunction|SpawnTile "0, 0, 0")))))

(fn SeedingArrayOfEnemyColours
  (params (NumberOfEnemies :type Integer) (UpcomingColour :type Integer))
  (bind _allcolours (Variables|Default|GetAllColours))
  (LocalVariables|SetNEnemies NumberOfEnemies)
  (LocalVariables|SetTotColoursNeeded (* (LocalVariables|GetNEnemies) (Variables|Default|GetMaxTilesWithEnemies)))
  (bind (_firstcolour _secondcolour) (CallFunction|Get2ColoursOfCombination UpcomingColour))
  (LocalVariables|SetColour1 _firstcolour)
  (LocalVariables|SetColour2 _secondcolour)
  (bind _resultnumberint (CallFunction|CalculatePercentageInt (Variables|Default|GetPercentageOfAppropriateEnemies) (LocalVariables|GetTotColoursNeeded)))
  (bind _output_get (LocalVariables|SetAppropriateNumberOfEnemiesForEachColour _resultnumberint))
  (for _index (range 1 _output_get)
    (Utilities|Array|Add _allcolours (LocalVariables|GetColour1))
    (Utilities|Array|Add _allcolours (LocalVariables|GetColour2)))
  (for _index_2 (range 1 (- (LocalVariables|GetTotColoursNeeded) (* (LocalVariables|GetAppropriateNumberOfEnemiesForEachColour) 2)))
    (Utilities|Array|Add (Variables|Default|GetAllColours) (Math|Random|RandomIntegerinRange 0 3)))
  (Utilities|Array|Shuffle (Variables|Default|GetAllColours)))

(fn Get2ColoursOfCombination
  (params (CombinedColour :type Integer))
  (switch int CombinedColour
    (:Default
      (LocalVariables|SetColour1 1 :!label _label)
      (LocalVariables|SetColour2 2))
    (:0
      (LocalVariables|SetColour1 1)
      (LocalVariables|SetColour2 3))
    (:1
      (LocalVariables|SetColour1 0)
      (LocalVariables|SetColour2 3))
    (:2
      (LocalVariables|SetColour1 0)
      (LocalVariables|SetColour2 1))
    (:3
      (LocalVariables|SetColour1 0)
      (LocalVariables|SetColour2 2))
    (:4
      (goto _label)))
  (return (LocalVariables|GetColour1) (LocalVariables|GetColour2)))

(fn CalculatePercentageInt
  (params (Percentage :type Float%20%28single-precision%29) (Number :type Integer))
  ;[1 1 1] Function to calculate percentage and convert to integer value
  (return (Math|Float|Round (/ (* Number Percentage) 1e+02))))