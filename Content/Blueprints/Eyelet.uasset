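; Eyelet is a touch point belonging to a tear that the player activates to progress that tear's closing.
; The first VeilCharacter overlap with its sphere flags it as touched, increments MyTear's touched count and calls UpdateClosingTear.
; The same one-shot event plays a random pool sound and recolours the dynamic material, created in the construction script, to the validation colour.
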(event OnComponentBeginOverlap(Sphere)
  (params (OverlappedComponent :type Primitive%20Component%20Object%20Reference) (OtherActor :type Actor%20Object%20Reference) (OtherComp :type Primitive%20Component%20Object%20Reference) (OtherBodyIndex :type Integer) (bFromSweep :type Boolean) (SweepResult :type Hit%20Result%20Structure%20%28by%20ref%29))
  (bind _mytear (Variables|Default|GetmyTear))
  (Utilities|Casting|CastToVeilCharacter OtherActor)
  (Utilities|FlowControl|DoOnce false ; If player has touched the eyelet, this will be flagged as overlapped and it will change oclour to tear oclour to indicate this operation
    (:Completed
      (Variables|Default|SethasBeenOverlapped true)
      (Math|Integer|IncrementInt (Variables|/Game/Blueprints/BaseTear.BaseTear_C|GetTouchedEyelets _mytear)
        (:%20%20
          (Default|UpdateClosingTear _mytear)
          (Audio|PlaySoundatLocation (Utilities|Array|Get(acopy) (Variables|Default|GetpoolSound) (Math|Random|RandomIntegerinRange 0 2)) (Transformation|GetActorLocation))
          (Rendering|Material|SetVectorParameterValue (Variables|Default|GetEyeletMaterial) "MyColor" (Variables|Default|GetEyeletValidationColour) :!class /Script/Engine.MaterialInstanceDynamic))))))

(event EventBeginPlay)

(event Collision|EventActorBeginOverlap
  (params (OtherActor :type Actor%20Object%20Reference)))

(event EventTick
  (params (DeltaSeconds :type Float%20%28single-precision%29)))

(fn ConstructionScript
  (bind _returnvalue (Rendering|Material|CreateDynamicMaterialInstance (Variables|Default|GeteyeletFB) 0 "/Game/Materials/Red.Red" :!class /Script/Engine.PrimitiveComponent)) ; Dynamic material to change colour of eyelet when touched
  (Variables|Default|SetEyeletMaterial _returnvalue))