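; Base 2D pickup actor that the player's VeilCharacter collects on overlap, with an empty PerformEffect hook for the pickup's effect.
; On spawn it caches the player, randomly decides whether it is upside down, negating Height if so, and destroys itself after a fixed lifetime.
; A gated box overlap runs the effect, plays a sound, swaps and rescales the flipbook with collision off, then destroys the actor when the animation ends.
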(event OnComponentBeginOverlap(Box)
  (params (OverlappedComponent :type Primitive%20Component%20Object%20Reference) (OtherActor :type Actor%20Object%20Reference) (OtherComp :type Primitive%20Component%20Object%20Reference) (OtherBodyIndex :type Integer) (bFromSweep :type Boolean) (SweepResult :type Hit%20Result%20Structure%20%28by%20ref%29))
  (Utilities|Casting|CastToVeilCharacter OtherActor)
  (Utilities|FlowControl|DoOnce false
    (:Completed
      (CallFunction|PerformEffect)
      (Audio|PlaySound2D (Variables|Default|GetpickedSound))
      (bind _secondstodie (CallFunction|PickedAnimtion (Variables|Default|GetPickedAnimation)))
      (Utilities|FlowControl|Delay _secondstodie)
      (Actor|DestroyActor))))

(event OnComponentEndOverlap(Box)
  (params (OverlappedComponent :type Primitive%20Component%20Object%20Reference) (OtherActor :type Actor%20Object%20Reference) (OtherComp :type Primitive%20Component%20Object%20Reference) (OtherBodyIndex :type Integer))
  (Utilities|Casting|CastToVeilCharacter OtherActor)
  (Utilities|FlowControl|DoOnce false) ; enters at Reset
)

(event EventBeginPlay
  (Variables|Default|SetisUpsideDown (Math|Random|RandomBool))
  (bind _asveil_character (Utilities|Casting|CastToVeilCharacter (Game|GetPlayerCharacter 0)))
  (Variables|Default|SetThisCharacter _asveil_character)
  (if (Variables|Default|GetisUpsideDown)
    (Variables|Default|SetHeight (* -1 (Variables|Default|GetHeight))))
  (Utilities|FlowControl|Delay 3e+01)
  (Actor|DestroyActor))

(event Collision|EventActorBeginOverlap
  (params (OtherActor :type Actor%20Object%20Reference)))

(event EventTick
  (params (DeltaSeconds :type Float%20%28single-precision%29)))

(fn ConstructionScript)

(fn PerformEffect)

(fn PickedAnimtion
  (params (NewFlipBook :type Paper%20Flipbook%20Object%20Reference))
  (bind _paperflipbook (Variables|Default|GetPaperFlipbook))
  (Sprite|SetFlipbook _paperflipbook NewFlipBook)
  (Transformation|SetRelativeScale3D _paperflipbook (Variables|Default|GetNewScale))
  (Collision|SetCollisionEnabled (Variables|Default|GetBox) "NoCollision")
  (return (Class|PaperFlipbook|GetTotalDuration NewFlipBook)))