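; PickupSpawner randomly decides whether to place a health or error-bar-clear pickup ahead of the newest level tile.
; SpawnPickup picks a random X within a range derived from the TileSpawner's newest tile floor width and its enemy tile limit.
; DetermineTypePickup spawns a random pickup class at triple scale, then moves it to that X at the pickup's own Height.
; Its event graph is empty, so SpawnPickup relies on an external caller.
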(event EventBeginPlay)

(event Collision|EventActorBeginOverlap
  (params (OtherActor :type Actor%20Object%20Reference)))

(event EventTick
  (params (DeltaSeconds :type Float%20%28single-precision%29)))

(fn ConstructionScript)

(fn SpawnPickup
  (bind _tilespawnerref (Variables|Default|GetTileSpawnerRef))
  (bind _newesttile (Variables|/Game/Blueprints/Managers_and_Spawners/TileSpawner.TileSpawner_C|GetNewestTile _tilespawnerref))
  (bind _floor (Variables|/Game/Blueprints/BaseTile.BaseTile_C|GetFloor _newesttile))
  (bind _output_get (Variables|Default|SetshouldSpawn (Math|Random|RandomBool)))
  (if _output_get
    (LocalVariables|SetMinX (Math|Float|Truncate (+ (.x (Transformation|GetWorldLocation (Variables|/Script/Engine.Actor|GetRootComponent _newesttile))) (* (.x (.BoxExtent (Collision|GetComponentBounds _floor))) 2.0))))
    (LocalVariables|SetMaxX (+ (LocalVariables|GetMinX) (Math|Float|Truncate (* (* (.x (.BoxExtent (Collision|GetComponentBounds _floor))) 2.0) (Math|Conversions|ToFloat(Integer) (- (Variables|/Game/Blueprints/Managers_and_Spawners/TileSpawner.TileSpawner_C|GetMaxTilesWithEnemies _tilespawnerref) 2))))))
    (bind _output_get_2 (LocalVariables|SetXLocation (Math|Random|RandomIntegerinRange (LocalVariables|GetMinX) (LocalVariables|GetMaxX))))
    (CallFunction|DetermineTypePickup _output_get_2)))

(fn DetermineTypePickup
  (params (XLocation :type Integer))
  (LocalVariables|SetNewXLocation XLocation)
  (bind _output_get (Variables|Default|SetPickupToSpawn (Math|Random|RandomIntegerinRange 0 (- (Variables|Default|GetHowManyPickups) 1))))
  (bind _returnvalue (Game|SpawnActorfromClass (Utilities|Select :Index _output_get :Option%200 "/Game/Blueprints/HealthPickup.HealthPickup_C" :Option%201 "/Game/Blueprints/ErrorBarClearPickup.ErrorBarClearPickup_C") (Math|Transform|MakeTransform "0, 0, 0" "0, 0, 0" "3.000000,3.000000,3.000000") "Undefined" 0 0))
  (bind _asbase_pickup (Utilities|Casting|CastToBasePickup _returnvalue))
  (bind _output_get_2 (Variables|Default|SetCurrentPickup _asbase_pickup))
  (Utilities|IsValid _output_get_2
    (:Is%20Valid
      (Transformation|SetActorLocation _output_get_2 (Math|Vector|MakeVector (Math|Conversions|ToFloat(Integer) (LocalVariables|GetNewXLocation)) 0.0 (Variables|/Game/Blueprints/BasePickup.BasePickup_C|GetHeight _output_get_2)) false false))))