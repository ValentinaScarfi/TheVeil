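; Enemy spawner that picks X positions along a tile and spawns coloured GenericEnemy actors there, registering each with the tile.
; SpawnAlgorithm draws random positions at a minimum spacing, re-rolling on conflicts and falling back to even spacing when retries run out.
; Spawn randomly flips each enemy, seating it above or below the floor using collider and floor extents.
; SpawnTutorialEnemies returns a single random position without spacing checks.
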(event EventBeginPlay)

(event Collision|EventActorBeginOverlap
  (params (OtherActor :type Actor%20Object%20Reference)))

(event EventTick
  (params (DeltaSeconds :type Float%20%28single-precision%29)))

(fn ConstructionScript)

(fn Spawn
  (params (PositionX :type Integer) (SpawnEnemyColour :type Integer))
  (LocalVariables|SetNewEnemyColour SpawnEnemyColour)
  (bind _returnvalue (Game|SpawnActorfromClass "/Game/Blueprints/GenericEnemy.GenericEnemy_C" (Math|Transform|MakeTransform (Math|Vector|MakeVector (Math|Conversions|ToFloat(Integer) PositionX) 0.0 0.0) "0, 0, 0" "2.000000,2.000000,2.000000") "Undefined" 0 0))
  (Default|SetEnemyColour _returnvalue (LocalVariables|GetNewEnemyColour))
  (Variables|/Game/Blueprints/GenericEnemy.GenericEnemy_C|SetMySpawner _returnvalue self) ; Setting spawner of new spawned enemy to THIS
  (Default|SetUpsideDownEnemy _returnvalue (Math|Random|RandomBool))
  (bind _movedenemy (CallFunction|DetermineZPositionandOrientation _returnvalue))
  (Utilities|Array|Add (Variables|/Game/Blueprints/BaseTile.BaseTile_C|GetEnemies (Variables|Default|GetThisTile)) _movedenemy))

(fn DetermineZPositionandOrientation
  (params (Enemy :type Generic%20Enemy%20Object%20Reference))
  (bind _thistile (Variables|Default|GetThisTile))
  (bind _enemycollider (Variables|/Game/Blueprints/GenericEnemy.GenericEnemy_C|GetEnemyCollider Enemy))
  (bind _returnvalue (Components|Box|GetScaledBoxExtent _enemycollider))
  (bind _floor (Variables|/Game/Blueprints/BaseTile.BaseTile_C|GetFloor _thistile))
  (bind _relativelocation (Variables|/Script/Engine.SceneComponent|GetRelativeLocation _enemycollider))
  (bind _boxextent (Collision|GetComponentBounds _floor))
  (bind _returnvalue_2 (+ (.z _returnvalue) (.z _boxextent)))
  (if (Variables|/Game/Blueprints/GenericEnemy.GenericEnemy_C|GetisUpsideDown Enemy) ; Check if generated enemy should be upside down
    (Transformation|SetActorRelativeLocation Enemy (Math|Vector|MakeVector (.x _relativelocation) (.y _relativelocation) (* _returnvalue_2 -1.0)))
    (else
      (Transformation|SetActorRelativeLocation Enemy (Math|Vector|MakeVector (.x _relativelocation) (.y _relativelocation) _returnvalue_2))))
  (return Enemy))

(fn SpawnAlgorithm
  (params (NumberOfEnemiesEachTile :type Integer) (MinimumDistanceBetweenEnemies :type Integer))
  (LocalVariables|SetEnemiesPerTile NumberOfEnemiesEachTile)
  (LocalVariables|SetMinDistance MinimumDistanceBetweenEnemies)
  (for _index (range 0 (- (LocalVariables|GetEnemiesPerTile) 1))
    (if (== (LocalVariables|GetcurrentRandomX) -300000) ; If current X is -300000, then first it is the first enemy to create on current tile
      (bind _randominrangeoftile (CallFunction|RandomNumberinTileRange 2400 -2400 (LocalVariables|GetMinDistance)))
      (bind _output_get (LocalVariables|SetcurrentRandomX _randominrangeoftile))
      (bind _result (CallFunction|AddSpawnPointPos _output_get))
      (Utilities|Array|Add (Variables|Default|GetEnemiesPositions) _result)
      (else
        (bind _randominrangeoftile_2 (CallFunction|RandomNumberinTileRange 2400 -2400 (LocalVariables|GetMinDistance)))
        (LocalVariables|SetcurrentRandomX _randominrangeoftile_2)
        (for _array_element (Variables|Default|GetEnemiesPositions)
          (bind _result_2 (CallFunction|AddSpawnPointPos (LocalVariables|GetcurrentRandomX)))
          (bind _isinrange (CallFunction|IsRandominRange _result_2 _array_element (LocalVariables|GetMinDistance)))
          (bind _output_get_2 (LocalVariables|SetisNewXInRange _isinrange))
          (LocalVariables|SetloopCount 0)
          (while _output_get_2
            (bind _result_3 (Math|Integer|IncrementInt (LocalVariables|GetloopCount))
              (:%20%20
                (if (>= _result_3 20)
                  (LocalVariables|SetisNewXInRange false)
                  (LocalVariables|SetnoSolutionFound true)
                  (else
                    (LocalVariables|SetnoSolutionFound false)
                    (bind _randominrangeoftile_3 (CallFunction|RandomNumberinTileRange 2400 -2400 (LocalVariables|GetMinDistance)))
                    (bind _output_get_3 (LocalVariables|SetcurrentRandomX _randominrangeoftile_3))
                    (bind _result_4 (CallFunction|AddSpawnPointPos _output_get_3))
                    (for _array_element_2 (Variables|Default|GetEnemiesPositions)
                      (bind _isinrange_2 (CallFunction|IsRandominRange _result_4 _array_element_2 (LocalVariables|GetMinDistance)))
                      (Utilities|Array|Add (LocalVariables|GetallPointsOutRange) _isinrange_2))
                    (LocalVariables|SetisNewXInRange (Utilities|Array|ContainsItem (LocalVariables|GetallPointsOutRange) true))
                    (Utilities|Array|Clear (LocalVariables|GetallPointsOutRange))))))))
        (bind _result_5 (CallFunction|AddSpawnPointPos (LocalVariables|GetcurrentRandomX)))
        (Utilities|Array|Add (Variables|Default|GetEnemiesPositions) _result_5))))
  (LocalVariables|SetcurrentRandomX -300000)
  (if (LocalVariables|GetnoSolutionFound)
    (CallFunction|GetDefaultEnemiesPos (LocalVariables|GetEnemiesPerTile) (LocalVariables|GetMinDistance))))

(fn IsRandominRange
  (params (NewIntToCheck :type Integer) (BaseInt :type Integer) (Range :type Integer))
  (return (and (<= NewIntToCheck (+ BaseInt Range)) (>= NewIntToCheck (- BaseInt Range)))))

(fn AddSpawnPointPos
  (params (IntToAddToSpawnPos :type Integer))
  (return (+ IntToAddToSpawnPos (Math|Float|Truncate (.x (Transformation|GetWorldLocation (Variables|/Game/Blueprints/BaseTile.BaseTile_C|GetEnemySpawnOrigin (Variables|Default|GetThisTile))))))))

(fn GetMinRange
  (params (Range :type Integer) (HalfTileMin :type Integer))
  (return (+ HalfTileMin (/ Range 2))))

(fn RandomNumberinTileRange
  (params (PositiveTileEnd :type Integer) (NegativeTileEnd :type Integer) (Range :type Integer))
  (bind _newminrange (CallFunction|GetMinRange Range NegativeTileEnd))
  (bind _newmaxrange (CallFunction|GetMaxRange Range PositiveTileEnd))
  (return (Math|Random|RandomIntegerinRange _newminrange _newmaxrange)))

(fn GetMaxRange
  (params (Range :type Integer) (HalfTileRange :type Integer))
  (return (- HalfTileRange (/ Range 2))))

(fn GetDefaultEnemiesPos
  (params (NumberOfEnemies :type Integer) (MinDistance :type Integer))
  (LocalVariables|SetNEnemies NumberOfEnemies)
  (Utilities|Array|Clear (Variables|Default|GetEnemiesPositions))
  (LocalVariables|SetDistanceForDefaultEnemies (/ (- (LocalVariables|GetTileLength) MinDistance) (LocalVariables|GetNEnemies)))
  (LocalVariables|SetCurrentLastPosition (+ (LocalVariables|GetStartingPointToAddPositions) (/ (LocalVariables|GetDistanceForDefaultEnemies) 2)))
  (for _index (range 1 (LocalVariables|GetNEnemies))
    (bind _output_get (LocalVariables|SetCurrentLastPosition (+ (LocalVariables|GetCurrentLastPosition) (LocalVariables|GetDistanceForDefaultEnemies))))
    (bind _result (CallFunction|AddSpawnPointPos _output_get))
    (Utilities|Array|Add (Variables|Default|GetEnemiesPositions) _result)))

(fn SpawnTutorialEnemies
  (params (MinimumDistance :type Integer))
  (bind _output_get (LocalVariables|SetMinDist MinimumDistance))
  (bind _randominrangeoftile (CallFunction|RandomNumberinTileRange 2400 -2400 _output_get))
  (bind _result (CallFunction|AddSpawnPointPos _randominrangeoftile))
  (return _result))