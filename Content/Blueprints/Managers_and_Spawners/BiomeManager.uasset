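; BiomeManager switches the active biome among three options and sets which tile pool is current.
; ChangeBiome resets TearsToNextBiome, currently always 1 because the random range is fixed, then calls SelectBiome.
; SelectBiome rerolls until the biome differs from the current one, then SetPoolOfTiles copies that biome's tile list into CurrentPoolTiles.
; Event graph and construction script are empty, and nothing here calls ChangeBiome.
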(event EventBeginPlay)

(event Collision|EventActorBeginOverlap
  (params (OtherActor :type Actor%20Object%20Reference)))

(event EventTick
  (params (DeltaSeconds :type Float%20%28single-precision%29)))

(fn ConstructionScript)

(fn SetTearstoNextBiome
  (Variables|Default|SetTearsToNextBiome (Math|Random|RandomIntegerinRange 1 1)))

(fn SelectBiome
  (bind _output_get (LocalVariables|SetNewBiome (Math|Random|RandomIntegerinRange 0 2)))
  (if (== _output_get (Variables|Default|GetCurrentBiome)) :!label _label
    (LocalVariables|SetNewBiome (Math|Random|RandomIntegerinRange 0 2))
    (goto _label)
    (else
      (bind _output_get_2 (Variables|Default|SetCurrentBiome (LocalVariables|GetNewBiome)))
      (CallFunction|SetPoolOfTiles _output_get_2))))

(fn SetPoolOfTiles
  (params (BiomeID :type Integer))
  (Utilities|Array|Clear (Variables|Default|GetCurrentPoolTiles))
  (switch int BiomeID
    (:Default
      (Variables|Default|SetCurrentPoolTiles (Variables|Default|GetallBiome1Tiles) :!label _label))
    (:0
      (goto _label))
    (:1
      (Variables|Default|SetCurrentPoolTiles (Variables|Default|GetallBiome2Tiles)))
    (:2
      (Variables|Default|SetCurrentPoolTiles (Variables|Default|GetallBiome3Tiles)))))

(fn ChangeBiome
  (CallFunction|SetTearstoNextBiome)
  (CallFunction|SelectBiome))