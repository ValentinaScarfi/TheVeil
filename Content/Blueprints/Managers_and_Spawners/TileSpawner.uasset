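; Tile spawner that builds the level by chaining random tiles from the current biome's pool at the newest tile's spawn point.
; It periodically makes a tear tile with a tear and pickup, advancing the biome after enough tears.
; Other tiles get enemies from a shuffled colour pool seeded with the two components of the tear's mixed colour, which tile indicators display.
; During tutorials, TutorialManager state drives enemy colours and tear spawns.
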(event EventBeginPlay
  (Variables|Default|SetCurrentColourOfTear 7) ; Setting first random colour of tear
  (Default|ChangeBiome (Variables|Default|GetBiomeManagerRef))
  (CallFunction|SpawnInitialTiles))

(event Collision|EventActorBeginOverlap
  (params (OtherActor :type Actor%20Object%20Reference)))

(event EventTick
  (params (DeltaSeconds :type Float%20%28single-precision%29)))

(fn ConstructionScript)

(fn SpawnTile
  (params (SpawnLocation :type Vector))
  (bind _returnvalue (Game|SpawnActorfromClass (Utilities|Array|Get(acopy) (Variables|/Game/Blueprints/Managers_and_Spawners/BiomeManager.BiomeManager_C|GetCurrentPoolTiles (Variables|Default|GetBiomeManagerRef)) (Math|Random|RandomIntegerinRange 0 (- (Utilities|Array|Length (Variables|/Game/Blueprints/Managers_and_Spawners/BiomeManager.BiomeManager_C|GetCurrentPoolTiles (Variables|Default|GetBiomeManagerRef))) 1))) (Math|Transform|MakeTransform SpawnLocation "0, 0, 0" "50.000000,2.000000,1.000000") "Undefined" 0 0))
  (bind _asbase_tile (Utilities|Casting|CastToBaseTile _returnvalue))
  (bind _output_get (Variables|Default|SetNewestTile _asbase_tile))
  (Variables|/Game/Blueprints/BaseTile.BaseTile_C|SetTileSpawner _output_get self)
  (CallFunction|SetTileColourIndicators (Variables|Default|GetCurrentColourOfTear))
  (bind _asveil_character (Utilities|Casting|CastToVeilCharacter (Game|GetPlayerCharacter 0)))
  (Variables|/Game/Blueprints/VeilCharacter.VeilCharacter_C|SetInitialTile _asveil_character (Variables|Default|GetNewestTile))
  (if (> (Variables|Default|GetCounterToTearTile) (Variables|Default|GetMaxTilesWithEnemies))
    (Variables|/Game/Blueprints/BaseTile.BaseTile_C|SetisTearTile (Variables|Default|GetNewestTile) true)
    (Variables|Default|SetCounterToTearTile 0) ; Resetting counter after tear
  ))

(fn SpawnTileatSpawnPoint
  (bind _tearspawnerref (Variables|Default|GetTearSpawnerRef))
  (bind _biomemanagerref (Variables|Default|GetBiomeManagerRef))
  (bind _newesttile (Variables|Default|GetNewestTile))
  (bind _enemyspawnerref (Variables|Default|GetEnemySpawnerRef))
  (bind _newesttile_2 (Variables|Default|GetNewestTile))
  (bind _currenttear (Variables|/Game/Blueprints/Managers_and_Spawners/TearSpawner.TearSpawner_C|GetCurrentTear _tearspawnerref))
  (bind _spawnpoint (Variables|/Game/Blueprints/BaseTile.BaseTile_C|GetSpawnPoint _newesttile))
  (bind _returnvalue (Transformation|GetWorldLocation _spawnpoint))
  ;[1 1 1] Spawning a new tile at spawning point defined in Tile class
  (if (Variables|/Game/Blueprints/Managers_and_Spawners/TutorialManager.TutorialManager_C|GetisTutorialActive (Variables|Default|GetTutorialManagerRef))
    _
    (elif (== (Variables|Default|GetCounterToTearTile) 1)
      (bind _output_get (Variables|Default|SetNewColourOfTear (Math|Random|RandomIntegerinRange 0 4)))
      (if (== _output_get (Variables|Default|GetCurrentColourOfTear)) :!label _label
        (Variables|Default|SetNewColourOfTear (Math|Random|RandomIntegerinRange 0 4))
        (goto _label)
        (else
          (Variables|Default|SetCurrentColourOfTear (Variables|Default|GetNewColourOfTear))))))
  ;[1 1 1] Set next colour when counter of tiles reaches defined values
  (CallFunction|SpawnTile (Math|Vector|MakeVector (+ (.x (.BoxExtent (Collision|GetComponentBounds (Variables|/Game/Blueprints/BaseTile.BaseTile_C|GetFloor _newesttile)))) (.x _returnvalue)) (.y _returnvalue) (.z _returnvalue)))
  (if (Variables|/Game/Blueprints/Managers_and_Spawners/TutorialManager.TutorialManager_C|GetisTutorialActive (Variables|Default|GetTutorialManagerRef))
    (CallFunction|TutorialTilesSpawn)
    (else
      (Math|Integer|IncrementInt (Variables|Default|GetCounterToTearTile)
        (:%20%20
          ;[1 1 1] Setting current tile of enemy spawner and spawn new enemy - function is called here to avoid enemies to first tile spawned in world. Spawn algorithm determines random positions of enemies, spawn functions spawns all he enemies at the determined positions
          (Variables|/Game/Blueprints/Managers_and_Spawners/EnemySpawner.EnemySpawner_C|SetThisTile (Variables|Default|GetEnemySpawnerRef) _newesttile_2 :!pinned true) ; When new tile is spawned, the current "ThisTile" in spawner is set to newest tile spawned, to allow new enemies to spawn on it
          (if (Variables|/Game/Blueprints/BaseTile.BaseTile_C|GetisTearTile _newesttile_2)
            ;[1 1 1] Spawn tear on tear tile and set its colour, based on current colour
            (Math|Integer|IncrementInt (Variables|/Game/Blueprints/Managers_and_Spawners/BiomeManager.BiomeManager_C|GetCounterToNextBiome (Variables|Default|GetBiomeManagerRef))
              (:%20%20
                (Default|SpawnTear _tearspawnerref)
                (Variables|/Game/Blueprints/BaseTile.BaseTile_C|SetmyTear (Variables|Default|GetNewestTile) _currenttear)
                (Variables|/Game/Blueprints/BaseTear.BaseTear_C|SetTearColour _currenttear (Variables|Default|GetCurrentColourOfTear))
                (Default|SetTearColour _currenttear)
                (Default|SetTearTexture _currenttear)
                (Default|SpawnPickup (Variables|Default|GetPickupSpawnerRef))
                (if (>= (Variables|/Game/Blueprints/Managers_and_Spawners/BiomeManager.BiomeManager_C|GetCounterToNextBiome _biomemanagerref) (Variables|/Game/Blueprints/Managers_and_Spawners/BiomeManager.BiomeManager_C|GetTearsToNextBiome _biomemanagerref))
                  (Default|ChangeBiome _biomemanagerref))))
            (else
              (Variables|/Game/Blueprints/BaseTile.BaseTile_C|SetTileID (Variables|Default|GetNewestTile) (- (Variables|Default|GetCounterToTearTile) 1))
              (Default|SpawnAlgorithm _enemyspawnerref (Variables|Default|GetNumberOfEnemiesPerTile) (Variables|Default|GetMinDistanceEnemies)) ; Spawn n enemies at x positions
              ;[1 1 1] Seeding correct colour of enemies
              (if (== (Variables|Default|GetIndexOfArrayOfColours) 0)
                (CallFunction|SeedingArrayOfEnemyColours (Variables|Default|GetNumberOfEnemiesPerTile) (Variables|Default|GetCurrentColourOfTear)) ; Seeding enemies colours to be sure player has the chance to form the right combination
              )
              (for (_array_element _array_index) (Variables|/Game/Blueprints/Managers_and_Spawners/EnemySpawner.EnemySpawner_C|GetEnemiesPositions _enemyspawnerref)
                (Default|Spawn (Variables|Default|GetEnemySpawnerRef) _array_element (Utilities|Array|Get(acopy) (Variables|Default|GetAllColours) (+ _array_index (* (Variables|Default|GetIndexOfArrayOfColours) (Variables|Default|GetNumberOfEnemiesPerTile))))))
              (Utilities|Array|Clear (Variables|/Game/Blueprints/Managers_and_Spawners/EnemySpawner.EnemySpawner_C|GetEnemiesPositions (Variables|Default|GetEnemySpawnerRef))) ; Clear enemies positions to not overlap with new ones
              (if (== (Variables|/Game/Blueprints/BaseTile.BaseTile_C|GetTileID (Variables|Default|GetNewestTile)) (Variables|Default|GetMaxTilesWithEnemies))
                (Utilities|Array|Clear (Variables|Default|GetAllColours)) ; Array of colour is cleared as all the colours have been used
                (Variables|Default|SetIndexOfArrayOfColours 0)
                (else
                  (bind _result (Math|Integer|IncrementInt (Variables|Default|GetIndexOfArrayOfColours)) ; Index of colours increases as last tile with enemies has not been reached yet
                    (:%20%20
                      (Variables|Default|SetIndexOfArrayOfColours _result))))))))))))

(fn SpawnInitialTiles
  ;[1 1 1] Tile Spawner - if first tile doesn't exist, spawns it at player location, followed by another tile at the spawn point
  (for _index (range 0 2)
    (Utilities|IsValid (Variables|Default|GetNewestTile)
      (:Is%20Valid
        (CallFunction|SpawnTileatSpawnPoint))
      (:Is%20Not%20Valid
        (CallFunction|SpawnTile "0, 0, 0")
        (Math|Integer|IncrementInt (Variables|Default|GetCounterToTearTile))))))

(fn SeedingArrayOfEnemyColours
  (params (NumberOfEnemies :type Integer) (UpcomingColour :type Integer))
  (bind _allcolours (Variables|Default|GetAllColours))
  (LocalVariables|SetNEnemies NumberOfEnemies)
  (LocalVariables|SetTotColoursNeeded (* (LocalVariables|GetNEnemies) (Variables|Default|GetMaxTilesWithEnemies)))
  (bind (_firstcolour _secondcolour) (CallFunction|Get2ColoursOfCombination UpcomingColour))
  (LocalVariables|SetColour1 _firstcolour)
  (LocalVariables|SetColour2 _secondcolour)
  (bind _resultnumberint (CallFunction|CalculatePercentageInt (Variables|Default|GetPercentageOfAppropriateEnemies) (LocalVariables|GetTotColoursNeeded)))
  (bind _output_get (LocalVariables|SetAppropriateNumberOfEnemiesForEachColour _resultnumberint))
  (for _index (range 1 _output_get)
    (Utilities|Array|Add _allcolours (LocalVariables|GetColour1))
    (Utilities|Array|Add _allcolours (LocalVariables|GetColour2)))
  (for _index_2 (range 1 (- (LocalVariables|GetTotColoursNeeded) (* (LocalVariables|GetAppropriateNumberOfEnemiesForEachColour) 2)))
    (Utilities|Array|Add (Variables|Default|GetAllColours) (Math|Random|RandomIntegerinRange 0 3)))
  (Utilities|Array|Shuffle (Variables|Default|GetAllColours)))

(fn Get2ColoursOfCombination
  (params (CombinedColour :type Integer))
  (switch int CombinedColour
    (:Default
      (LocalVariables|SetColour1 2)
      (LocalVariables|SetColour2 2))
    (:0
      (LocalVariables|SetColour1 1)
      (LocalVariables|SetColour2 3))
    (:1
      (LocalVariables|SetColour1 0)
      (LocalVariables|SetColour2 3))
    (:2
      (LocalVariables|SetColour1 0)
      (LocalVariables|SetColour2 1))
    (:3
      (LocalVariables|SetColour1 0)
      (LocalVariables|SetColour2 2))
    (:4
      (LocalVariables|SetColour1 1)
      (LocalVariables|SetColour2 2)))
  (return (LocalVariables|GetColour1) (LocalVariables|GetColour2)))

(fn CalculatePercentageInt
  (params (Percentage :type Float%20%28single-precision%29) (Number :type Integer))
  ;[1 1 1] Function to calculate percentage and convert to integer value
  (return (Math|Float|Round (/ (* Number Percentage) 1e+02))))

(fn TutorialTilesSpawn
  (bind _tearspawnerref (Variables|Default|GetTearSpawnerRef))
  (bind _tutorialmanagerref (Variables|Default|GetTutorialManagerRef))
  (bind _enemyspawnerref (Variables|Default|GetEnemySpawnerRef))
  (bind _tutorialmanagerref_2 (Variables|Default|GetTutorialManagerRef))
  (bind _currenttear (Variables|/Game/Blueprints/Managers_and_Spawners/TearSpawner.TearSpawner_C|GetCurrentTear _tearspawnerref))
  (if (Variables|/Game/Blueprints/Managers_and_Spawners/TutorialManager.TutorialManager_C|GetnoEnemiesNeeded _tutorialmanagerref)
    (Math|Integer|IncrementInt (Variables|Default|GetCurrentTutorialTile)
      (:%20%20
        (if (Variables|/Game/Blueprints/Managers_and_Spawners/TutorialManager.TutorialManager_C|GetisTip4 _tutorialmanagerref_2)
          (if (Variables|/Game/Blueprints/Managers_and_Spawners/TutorialManager.TutorialManager_C|GetisTearNeeded _tutorialmanagerref_2)
            (Default|SpawnTear _tearspawnerref)
            (Variables|/Game/Blueprints/BaseTile.BaseTile_C|SetmyTear (Variables|Default|GetNewestTile) _currenttear)
            (Variables|/Game/Blueprints/BaseTear.BaseTear_C|SetTearColour _currenttear (Variables|Default|GetCurrentColourOfTear))
            (Default|SetTearColour _currenttear)
            (Default|SetTearTexture _currenttear)
            (Variables|/Game/Blueprints/Managers_and_Spawners/TutorialManager.TutorialManager_C|SetisTearNeeded (Variables|Default|GetTutorialManagerRef) false)))))
    (else
      (Variables|Default|SetNewColourOfTear (Variables|/Game/Blueprints/Managers_and_Spawners/TutorialManager.TutorialManager_C|GetColourTutorial _tutorialmanagerref))
      (Variables|Default|SetCurrentColourOfTear (Variables|Default|GetNewColourOfTear))
      (if (< (Variables|Default|GetNTileOfEnemiesTutorial) 2)
        _
        (else
          (Variables|Default|SetNTileOfEnemiesTutorial 0)))
      (Math|Integer|IncrementInt (Variables|Default|GetNTileOfEnemiesTutorial)
        (:%20%20
          (Variables|/Game/Blueprints/Managers_and_Spawners/EnemySpawner.EnemySpawner_C|SetThisTile _enemyspawnerref (Variables|Default|GetNewestTile)) ; When new tile is spawned, the current "ThisTile" in spawner is set to newest tile spawned, to allow new enemies to spawn on it
          (bind _enemypos (Default|SpawnTutorialEnemies _enemyspawnerref 1000))
          (bind _enemycolour (CallFunction|SetTutorialColours (Variables|Default|GetCurrentColourOfTear) (Variables|Default|GetNTileOfEnemiesTutorial)))
          (Default|Spawn (Variables|Default|GetEnemySpawnerRef) _enemypos _enemycolour))))))

(fn SetTutorialColours
  (params (MixedColour :type Integer) (EnemyTile :type Integer))
  (bind (_firstcolour _secondcolour) (CallFunction|Get2ColoursOfCombination MixedColour))
  (switch int EnemyTile
    (:1
      (LocalVariables|SetOutputColour _firstcolour))
    (:2
      (LocalVariables|SetOutputColour _secondcolour)))
  (return (LocalVariables|GetOutputColour)))

(fn SetTileColourIndicators
  (params (CurrentColour :type Integer))
  (bind _output_get (LocalVariables|SetColour CurrentColour))
  (switch int _output_get ; Setting material colour according to int
    (:Default
      (LocalVariables|SetMiddleMixedColour ""))
    (:0
      (LocalVariables|SetMiddleMixedColour "(R=0.000392,G=0.100000,B=0.000000,A=1.000000)"))
    (:1
      (LocalVariables|SetMiddleMixedColour "(R=0.100000,G=0.032157,B=0.000000,A=1.000000)"))
    (:2
      (LocalVariables|SetMiddleMixedColour "(R=0.059216,G=0.000000,B=0.100000,A=1.000000)"))
    (:3
      (LocalVariables|SetMiddleMixedColour "(R=0.100000,G=0.018431,B=0.038823,A=1.000000)"))
    (:4
      (LocalVariables|SetMiddleMixedColour "(R=0.000000,G=0.097345,B=0.100000,A=1.000000)")))
  (Rendering|Material|SetVectorParameterValue (Variables|/Game/Blueprints/BaseTile.BaseTile_C|GetColourMiddleMat (Variables|Default|GetNewestTile)) "Mixed_COlour" (LocalVariables|GetMiddleMixedColour) :!class /Script/Engine.MaterialInstanceDynamic)
  (bind (_firstcolour _secondcolour) (CallFunction|Get2ColoursOfCombination (LocalVariables|GetColour)))
  (switch int _firstcolour
    (:Default
      (LocalVariables|SetTopColour ""))
    (:0
      (LocalVariables|SetTopColour "(R=0.100000,G=0.001961,B=0.000000,A=1.000000)"))
    (:1
      (LocalVariables|SetTopColour "(R=0.002290,G=0.000000,B=0.100000,A=1.000000)"))
    (:2
      (LocalVariables|SetTopColour "(R=0.098039,G=0.098039,B=0.098039,A=1.000000)"))
    (:3
      (LocalVariables|SetTopColour "(R=0.100000,G=0.082353,B=0.000000,A=1.000000)")))
  (Rendering|Material|SetVectorParameterValue (Variables|/Game/Blueprints/BaseTile.BaseTile_C|GetColourTopMat (Variables|Default|GetNewestTile)) "Top_Colour" (LocalVariables|GetTopColour) :!class /Script/Engine.MaterialInstanceDynamic)
  (switch int _secondcolour
    (:Default
      (LocalVariables|SetBottomColour ""))
    (:0
      (LocalVariables|SetBottomColour "(R=0.100000,G=0.000000,B=0.000000,A=1.000000)"))
    (:1
      (LocalVariables|SetBottomColour "(R=0.000000,G=0.000000,B=0.100000,A=1.000000)"))
    (:2
      (LocalVariables|SetBottomColour "(R=0.099899,G=0.099899,B=0.099899,A=1.000000)"))
    (:3
      (LocalVariables|SetBottomColour "(R=0.100000,G=0.082283,B=0.000000,A=1.000000)")))
  (Rendering|Material|SetVectorParameterValue (Variables|/Game/Blueprints/BaseTile.BaseTile_C|GetColourBottomMat (Variables|Default|GetNewestTile)) "Bottom_Colour" (LocalVariables|GetBottomColour) :!class /Script/Engine.MaterialInstanceDynamic))