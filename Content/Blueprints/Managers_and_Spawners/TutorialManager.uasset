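; TutorialManager runs Veil's step-by-step tutorial, from flipping, jumping, teleporting and attacking to colour mixing and tears.
; BeginPlay links it to the character and a new TutorialHUD, reading the active state from the game instance.
; Tick polls counters and flags to advance CurrentTip, with retry branches for failures.
; Named timers delay each tip's flags and side effects, like clearing enemies, and EndTutorial saves completion to the game instance.
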(event EventBeginPlay
  (bind _asveil_game_instance (Utilities|Casting|CastToVeilGameInstance (Game|GetGameInstance)))
  (Variables|TutorialStates|SetisTutorialActive (Variables|/Game/Blueprints/VeilGameInstance.VeilGameInstance_C|GetisTutorialActive _asveil_game_instance))
  (bind _asveil_character (Utilities|Casting|CastToVeilCharacter (Game|GetPlayerCharacter 0)))
  (bind _output_get (Variables|ExternalRef|SetThisCharacter _asveil_character))
  (Variables|/Game/Blueprints/VeilCharacter.VeilCharacter_C|SetTutorialManagerRef _output_get self)
  (bind _returnvalue (UserInterface|CreateWidget "/Game/UI/CharacterHUD/TutorialHUD.TutorialHUD_C" (Game|GetPlayerController 0)))
  (UserInterface|Viewport|AddtoViewport _returnvalue 0)
  (bind _output_get_2 (Variables|ExternalRef|SetTutorialHUD _returnvalue))
  (Variables|/Game/UI/CharacterHUD/TutorialHUD.TutorialHUD_C|SetTutorialManager _output_get_2 self)
  (Variables|TutorialValues|SetColourTutorial (Math|Random|RandomIntegerinRange 0 4)))

(event Collision|EventActorBeginOverlap
  (params (OtherActor :type Actor%20Object%20Reference)))

(event EventTick
  (params (DeltaSeconds :type Float%20%28single-precision%29))
  (if (Variables|TutorialStates|GetisTutorialActive)
    (CallFunction|ConditiontoProgressTutorial)))

(fn ConstructionScript)

(fn Tutorial
  (switch int (Variables|TutorialValues|GetCurrentTip)
    (:1
      (Variables|TutorialStates|SetnoEnemiesNeeded true)
      (Utilities|Time|SetTimerbyFunctionName 0 "Tip1Flip" 2.0))
    (:2
      (Utilities|Time|SetTimerbyFunctionName 0 "Tip2Jump" 2.0))
    (:3
      (Utilities|Time|SetTimerbyFunctionName 0 "Tip3Teleport" 2.0))
    (:4
      (Utilities|Time|SetTimerbyFunctionName 0 "Tip4Attack" 2.0))
    (:5
      (Utilities|Time|SetTimerbyFunctionName 0 "Tip5KillEnemy" 2.0))
    (:6
      (Utilities|Time|SetTimerbyFunctionName 0 "Tip5Failed" 0.5))
    (:7
      (Variables|TutorialStates|SetnoEnemiesNeeded false)
      (Utilities|Time|SetTimerbyFunctionName 0 "Tip7AbsorbAndMix" 0.5))
    (:8
      (Variables|TutorialStates|SetnoEnemiesNeeded false)
      (Utilities|Time|SetTimerbyFunctionName 0 "Tip8MixedColourReset" 0.5))
    (:9
      (Variables|TutorialStates|SetnoEnemiesNeeded false)
      (Utilities|Time|SetTimerbyFunctionName 0 "Tip9NextColour" 0.5))
    (:10
      (Utilities|Time|SetTimerbyFunctionName 0 "Tip10Tear" 0.5))
    (:11
      (Utilities|Time|SetTimerbyFunctionName 0 "Tip11TutorialComplete" 0.1))
    (:12
      (Utilities|Time|SetTimerbyFunctionName 0 "Tip12MissedTear" 0.5))))

(fn Tip1Flip
  (Variables|TutorialStates|SetisTip1 true))

(fn ResetBools
  (switch int (Variables|TutorialValues|GetCurrentTip)
    (:1
      (Variables|TutorialStates|SetisTip1 false))
    (:2
      (Variables|TutorialStates|SetisTip2 false))
    (:3
      (Variables|TutorialStates|SetisTip3 false))
    (:4
      (Variables|TutorialStates|SetisTip4 false))
    (:5
      (Variables|TutorialStates|SetisTip5 false)
      (Variables|TutorialStates|SetnoEnemiesNeeded true :!label _label))
    (:6
      (Variables|TutorialStates|SetisTip5Failed false)
      (goto _label))
    (:7
      (Variables|TutorialStates|SetisTip7 false)
      (Variables|TutorialStates|SetmixedColour false)
      (goto _label))
    (:8
      (Variables|TutorialStates|SetisTip8 false))
    (:9
      (Variables|TutorialStates|SetisTip9 false)
      (goto _label))
    (:10
      (Variables|TutorialStates|SetisTip10 false)
      (Variables|TutorialStates|SetMissedTear false :!label _label_2)
      (Variables|TutorialStates|SetCompletedTear false)
      (goto _label))
    (:11
      (Variables|TutorialStates|SetisTip11 false))
    (:12
      (Variables|TutorialStates|SetisTip12 false)
      (goto _label_2))))

(fn ConditiontoProgressTutorial
  (switch int (Variables|TutorialValues|GetCurrentTip)
    (:1
      (if (== (Variables|TutorialValues|GettimesFlipped) 6)
        (CallFunction|ResetBools :!label _label)
        (Math|Integer|IncrementInt (Variables|TutorialValues|GetCurrentTip)
          (:%20%20
            (CallFunction|Tutorial)))))
    (:2
      (if (== (Variables|TutorialValues|GettimesJumped) 6)
        (goto _label)))
    (:3
      (if (== (Variables|TutorialValues|GettimesTeleported) 10)
        (goto _label)))
    (:4
      (if (== (Variables|TutorialValues|GettimesAttacked) 4)
        (goto _label)))
    (:5
      (if (Variables|TutorialStates|GethasEnemyBeenAttacked)
        (CallFunction|ResetBools)
        (Math|Integer|IncrementInt (Variables|TutorialValues|GetCurrentTip)
          (:%20%20
            (goto _label)))
        (elif (Variables|TutorialStates|GethasPlayerLostHeart)
          (Variables|TutorialValues|SetCurrentTip 6)
          (CallFunction|Tutorial))))
    (:6
      (if (Variables|TutorialStates|GethasEnemyBeenAttacked)
        (goto _label)))
    (:7
      (if (Variables|TutorialStates|GetmixedColour) :!label _label_2
        (goto _label)))
    (:8
      (if (Variables|TutorialStates|GetresetColourMixed)
        (goto _label)))
    (:9
      (goto _label_2))
    (:10
      (if (Variables|TutorialStates|GetCompletedTear)
        (goto _label)
        (else
          (if (Variables|TutorialStates|GetMissedTear) :!label _label_3
            (Variables|TutorialStates|SetisTearNeeded true)
            (CallFunction|ResetBools)
            (Variables|TutorialValues|SetCurrentTip 12)
            (CallFunction|Tutorial)))))
    (:12
      (if (Variables|TutorialStates|GetCompletedTear)
        (CallFunction|ResetBools)
        (Variables|TutorialValues|SetCurrentTip 11)
        (CallFunction|Tutorial)
        (else
          (goto _label_3))))))

(fn Tip2Jump
  (Variables|TutorialStates|SetisTip2 true))

(fn Tip3Teleport
  (Variables|TutorialStates|SetisTip3 true))

(fn Tip4Attack
  (Variables|TutorialStates|SetisTip4 true))

(fn Tip5KillEnemy
  (Variables|TutorialStates|SetisTip5 true)
  (Variables|TutorialStates|SetnoEnemiesNeeded false))

(fn Tip5Failed
  (Variables|TutorialStates|SetisTip5 false)
  (Variables|TutorialStates|SetisTip5Failed true)
  (Variables|TutorialStates|SetnoEnemiesNeeded false))

(fn Tip7AbsorbandMix
  (Variables|TutorialStates|SetisPausingTip true)
  (Variables|TutorialStates|SetisTip7 true))

(fn Tip8MixedColourReset
  (Variables|TutorialStates|SetisPausingTip true)
  (Variables|TutorialStates|SetisTip8 true))

(fn Tip9NextColour
  (bind _thischaracter (Variables|ExternalRef|GetThisCharacter))
  (Variables|TutorialStates|SetisPausingTip true)
  (Variables|TutorialStates|SetisTip9 true)
  (Rendering|Material|SetVectorParameterValue (Variables|/Game/Blueprints/VeilCharacter.VeilCharacter_C|GetAbsorbedColourMat _thischaracter) "AbsorbedColour" "(R=0.000000,G=0.000000,B=0.000000,A=1.000000)" :!class /Script/Engine.MaterialInstanceDynamic) ; Resetting colour indicator to black after tear has passed
  (Utilities|Array|Clear (Variables|/Game/Blueprints/VeilCharacter.VeilCharacter_C|GetCurrentColoursAbsorbed _thischaracter)))

(fn Tip10Tear
  (Variables|TutorialStates|SetisPausingTip true)
  (Variables|TutorialStates|SetisTip10 true)
  (bind _outactors (Actor|GetAllActorsOfClass "/Game/Blueprints/GenericEnemy.GenericEnemy_C"))
  (for _array_element _outactors
    (Actor|DestroyActor _array_element)))

(fn Tip11TutorialComplete
  (bind _thischaracter (Variables|ExternalRef|GetThisCharacter))
  (Variables|/Game/Blueprints/VeilCharacter.VeilCharacter_C|SetHealthCurrent _thischaracter (Variables|/Game/Blueprints/VeilCharacter.VeilCharacter_C|GetHealthBase _thischaracter))
  (Default|UpdateHealth (Variables|/Game/Blueprints/VeilCharacter.VeilCharacter_C|GetHUD _thischaracter))
  (Variables|TutorialStates|SetisTip11 true))

(fn Tip12MissedTear
  (Variables|TutorialStates|SetisPausingTip true)
  (Variables|TutorialStates|SetisTip12 true)
  (bind _outactors (Actor|GetAllActorsOfClass "/Game/Blueprints/GenericEnemy.GenericEnemy_C"))
  (for _array_element _outactors
    (Actor|DestroyActor _array_element)))

(fn EndTutorial
  (CallFunction|ResetBools)
  (bind _output_get (Variables|TutorialStates|SetisTutorialActive false))
  (bind _asveil_game_instance (Utilities|Casting|CastToVeilGameInstance (Game|GetGameInstance)))
  (Variables|/Game/Blueprints/VeilGameInstance.VeilGameInstance_C|SetisTutorialActive _asveil_game_instance _output_get))