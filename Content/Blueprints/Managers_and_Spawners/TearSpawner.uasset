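; Manager actor that spawns random tears on the newest tile from the current pool.
; On BeginPlay it maps textures under the Tears materials folder by name via the Asset Registry.
; It also fills six tiered class arrays from the Tears3–8 data tables, then has the difficulty manager set the pool.
; SpawnTear places a random pool class at TileSpawner's newest tile, storing it as CurrentTear with a back-reference.
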(event EventBeginPlay
  (for _array_element (.OutAssetData (Class|AssetRegistry|GetAssetsbyPath (Class|AssetRegistryHelpers|GetAssetRegistry) "/Game/Materials/Tears" true false))
    (bind _astexture (Utilities|Casting|CastToTexture (Class|AssetRegistryHelpers|GetAsset _array_element)))
    (Utilities|Map|Add (Variables|Default|GetallTearTextures) (Utilities|GetObjectName _astexture) _astexture))
  (bind _outrownames (DataTable|GetDataTableRowNames "/Game/Blueprints/DifficultyStructures/Tears3.Tears3"))
  (for _array_element_2 _outrownames
    (bind _returnvalue (Utilities|GetDataTableRow "/Game/Blueprints/DifficultyStructures/Tears3.Tears3" _array_element_2)
      (:then
        (Utilities|Array|Add (Variables|Default|GetTear3Classes) (.actorclas _returnvalue)))))
  (bind _outrownames_2 (DataTable|GetDataTableRowNames "/Game/Blueprints/DifficultyStructures/Tears4.Tears4"))
  (for _array_element_3 _outrownames_2
    (bind _returnvalue_2 (Utilities|GetDataTableRow "/Game/Blueprints/DifficultyStructures/Tears4.Tears4" _array_element_3)
      (:then
        (Utilities|Array|Add (Variables|Default|GetTear4Classes) (.actorclas _returnvalue_2)))))
  (bind _outrownames_3 (DataTable|GetDataTableRowNames "/Game/Blueprints/DifficultyStructures/Tears5.Tears5"))
  (for _array_element_4 _outrownames_3
    (bind _returnvalue_3 (Utilities|GetDataTableRow "/Game/Blueprints/DifficultyStructures/Tears5.Tears5" _array_element_4)
      (:then
        (Utilities|Array|Add (Variables|Default|GetTear5Classes) (.actorclas _returnvalue_3)))))
  (bind _outrownames_4 (DataTable|GetDataTableRowNames "/Game/Blueprints/DifficultyStructures/Tears6.Tears6"))
  (for _array_element_5 _outrownames_4
    (bind _returnvalue_4 (Utilities|GetDataTableRow "/Game/Blueprints/DifficultyStructures/Tears6.Tears6" _array_element_5)
      (:then
        (Utilities|Array|Add (Variables|Default|GetTear6Classes) (.actorclas _returnvalue_4)))))
  (bind _outrownames_5 (DataTable|GetDataTableRowNames "/Game/Blueprints/DifficultyStructures/Tears7.Tears7"))
  (for _array_element_6 _outrownames_5
    (bind _returnvalue_5 (Utilities|GetDataTableRow "/Game/Blueprints/DifficultyStructures/Tears7.Tears7" _array_element_6)
      (:then
        (Utilities|Array|Add (Variables|Default|GetTear7Classes) (.actorclas _returnvalue_5)))))
  (bind _outrownames_6 (DataTable|GetDataTableRowNames "/Game/Blueprints/DifficultyStructures/Tears8.Tears8"))
  (for _array_element_7 _outrownames_6
    (bind _returnvalue_6 (Utilities|GetDataTableRow "/Game/Blueprints/DifficultyStructures/Tears8.Tears8" _array_element_7)
      (:then
        (Utilities|Array|Add (Variables|Default|GetTear8Classes) (.actorclas _returnvalue_6)))))
  (Default|SetTearPool (Variables|Default|GetDifficultyManagerRef)))

(event Collision|EventActorBeginOverlap
  (params (OtherActor :type Actor%20Object%20Reference)))

(event EventTick
  (params (DeltaSeconds :type Float%20%28single-precision%29)))

(fn ConstructionScript)

(fn SpawnTear
  (bind _output_get (LocalVariables|SetCurrentTearBlueprintIndex (Math|Random|RandomIntegerinRange 0 (- (Utilities|Array|Length (Variables|Default|GetCurrentTearsPool)) 1))))
  (bind _returnvalue (Game|SpawnActorfromClass (Utilities|Array|Get(acopy) (Variables|Default|GetCurrentTearsPool) _output_get) (Math|Transform|MakeTransform (Transformation|GetActorLocation (Variables|/Game/Blueprints/Managers_and_Spawners/TileSpawner.TileSpawner_C|GetNewestTile (Variables|Default|GetTileSpawnerRef))) "0, 0,90.000000" "50.000000,15.000000,1.000000") "Undefined" 0 0)) ; Spawning tear at latest tile location
  (bind _asbase_tear (Utilities|Casting|CastToBaseTear _returnvalue))
  (bind _output_get_2 (Variables|Default|SetCurrentTear _asbase_tear)) ; Setting current tear of spawner to current one
  (Variables|/Game/Blueprints/BaseTear.BaseTear_C|SetTearSpawnerRef _output_get_2 self))