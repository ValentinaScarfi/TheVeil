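; TutorialManager runs the player's tutorial tips, pausing the game when the first tip appears.
; On BeginPlay it registers itself with the VeilCharacter and creates a TutorialHUD widget that holds a reference back to it.
; Tutorial advances a tip counter and starts a short timer to Tip1Flip, which sets tip flags and pauses the game.
; ResetBools clears those flags without unpausing; only the first tip is implemented.
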(event EventBeginPlay
  (bind _asveil_character (Utilities|Casting|CastToVeilCharacter (Game|GetPlayerCharacter 0)))
  (bind _output_get (Variables|Default|SetThisCharacter _asveil_character))
  (Variables|/Game/Blueprints/VeilCharacter.VeilCharacter_C|SetTutorialManagerRef _output_get self)
  (bind _returnvalue (UserInterface|CreateWidget "/Game/UI/CharacterHUD/TutorialHUD.TutorialHUD_C" (Game|GetPlayerController 0)))
  (UserInterface|Viewport|AddtoViewport _returnvalue 0)
  (bind _output_get_2 (Variables|Default|SetTutorialHUD _returnvalue))
  (Variables|/Game/UI/CharacterHUD/TutorialHUD.TutorialHUD_C|SetTutorialManager _output_get_2 self))

(event Collision|EventActorBeginOverlap
  (params (OtherActor :type Actor%20Object%20Reference)))

(event EventTick
  (params (DeltaSeconds :type Float%20%28single-precision%29)))

(fn ConstructionScript)

(fn Tutorial
  (bind _result (Math|Integer|IncrementInt (Variables|Default|GetCurrentTip))
    (:%20%20
      (switch int _result
        (:1
          (Utilities|Time|SetTimerbyFunctionName 0 "Tip1Flip" 3.0))))))

(fn Tip1Flip
  (Variables|Default|SetisTip1 true)
  (Variables|Default|SetisAnyTip true)
  (bind _returnvalue (Game|SetGamePaused true))
  (Variables|Default|SetisPaused _returnvalue))

(fn ResetBools
  (switch int (Variables|Default|GetCurrentTip)
    (:1
      (Variables|Default|SetisTip1 false)
      (Variables|Default|SetisAnyTip false))))