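; Pickup Blueprint that clears one point from the character's error bar when its effect fires.
; PerformEffect decrements the character's ErrorTolerance only when it is above zero, guarded by a DoOnce, then calls UpdateErrorTolerance.
; The construction script runs the parent's, then sets the fairy-vanish pickup animation, heart pickup sound and a reduced scale.
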(event EventBeginPlay
  (|CallParentFunction) ; This node is disabled and will not be called.\nDrag off pins to build functionality.
)

(event Collision|EventActorBeginOverlap
  (params (OtherActor :type Actor%20Object%20Reference)))

(event EventTick
  (params (DeltaSeconds :type Float%20%28single-precision%29)))

(event EventPerformEffect
  (bind _thischaracter (Variables|Default|GetThisCharacter))
  (if (> (Variables|/Game/Blueprints/VeilCharacter.VeilCharacter_C|GeterrorTolerance _thischaracter) 0)
    (Utilities|FlowControl|DoOnce false
      (:Completed
        (Variables|/Game/Blueprints/VeilCharacter.VeilCharacter_C|SeterrorTolerance _thischaracter (- (Variables|/Game/Blueprints/VeilCharacter.VeilCharacter_C|GeterrorTolerance _thischaracter) 1))
        (Default|UpdateErrorTolerance _thischaracter)))))

(fn ConstructionScript
  (|CallParentFunction)
  (Variables|Default|SetPickedAnimation "/Game/Materials/Pickups/Animations/Error/fairyVanish_FB.fairyVanish_FB")
  (Variables|Default|SetNewScale "0.350000,0.350000,0.350000")
  (Variables|Default|SetpickedSound "/Game/Audio/SoundFX/Pickups/HeartPickup.HeartPickup"))