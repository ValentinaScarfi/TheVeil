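; Health pickup Blueprint, a child of a parent pickup class, that heals a character when its effect is performed.
; It overrides PerformEffect to call Heal on ThisCharacter, guarded by a DoOnce so healing fires only once.
; The construction script runs the parent's, then sets a heart-vanish flipbook as the picked animation and a small uniform scale.
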(event EventBeginPlay
  (|CallParentFunction) ; This node is disabled and will not be called.\nDrag off pins to build functionality.
)

(event Collision|EventActorBeginOverlap
  (params (OtherActor :type Actor%20Object%20Reference))
  (|CallParentFunction OtherActor) ; This node is disabled and will not be called.\nDrag off pins to build functionality.
)

(event EventTick
  (params (DeltaSeconds :type Float%20%28single-precision%29))
  (|CallParentFunction DeltaSeconds) ; This node is disabled and will not be called.\nDrag off pins to build functionality.
)

(event EventPerformEffect
  (Utilities|FlowControl|DoOnce false
    (:Completed
      (Default|Heal (Variables|Default|GetThisCharacter)))))

(fn ConstructionScript
  (|CallParentFunction)
  (Variables|Default|SetPickedAnimation "/Game/Materials/Pickups/Animations/Heart/HeartVanish_FB.HeartVanish_FB")
  (Variables|Default|SetNewScale "0.100000,0.100000,0.100000"))