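; Base tile actor for an endlessly spawned track that extends itself as the player character, VeilCharacter, moves through it.
; The first TriggerZone overlap by a living VeilCharacter has TileSpawner spawn the next tile.
; Outside the end game, the tile destroys itself after a delay, along with its tear and eyelets or its enemies.
; Construction creates dynamic materials for the top, middle and bottom colour meshes, intended for recolouring on eyelet touch.
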(event OnComponentBeginOverlap(TriggerZone)
  (params (OverlappedComponent :type Primitive%20Component%20Object%20Reference) (OtherActor :type Actor%20Object%20Reference) (OtherComp :type Primitive%20Component%20Object%20Reference) (OtherBodyIndex :type Integer) (bFromSweep :type Boolean) (SweepResult :type Hit%20Result%20Structure%20%28by%20ref%29))
  (bind _mytear (Variables|Default|GetmyTear))
  ;[1 1 1] Check collision, when TriggerZone is ovelapped by VeilCharacter, a new tile is spawn at the spawn point
  (bind _asveil_character (Utilities|Casting|CastToVeilCharacter OtherActor))
  (if (not (Variables|/Game/Blueprints/VeilCharacter.VeilCharacter_C|GetisDead _asveil_character))
    (Utilities|FlowControl|DoOnce false
      (:Completed
        (Default|SpawnTileatSpawnPoint (Variables|Default|GetTileSpawner)) ; Spawn next tile
        (bind _asveil_character_2 (Utilities|Casting|CastToVeilCharacter (Game|GetPlayerCharacter 0)))
        (if (not (Variables|/Game/Blueprints/VeilCharacter.VeilCharacter_C|GetisEndGame _asveil_character_2))
          (Utilities|FlowControl|Delay 6.0)
          (Actor|DestroyActor) ; Destroy this tile
          ;[1 1 1] If it is a tear tile, destroy eyelets and tear itslef too
          (if (Variables|Default|GetisTearTile)
            (for _array_element (Variables|/Game/Blueprints/BaseTear.BaseTear_C|GetEyelets _mytear)
              (Actor|DestroyActor _array_element))
            (Actor|DestroyActor _mytear)
            (else
              ;[1 1 1] Destroying all enemies on that tile to free memory
              (for _array_element_2 (Variables|Default|GetEnemies)
                (Utilities|IsValid _array_element_2
                  (:Is%20Valid
                    (Actor|DestroyActor _array_element_2)))))))))))

(event EventBeginPlay)

(event Collision|EventActorBeginOverlap
  (params (OtherActor :type Actor%20Object%20Reference)))

(event EventTick
  (params (DeltaSeconds :type Float%20%28single-precision%29)))

(fn ConstructionScript
  (bind _returnvalue (Rendering|Material|CreateDynamicMaterialInstance (Variables|Default|GetColourTopAurora) 0 "/Game/Materials/Environment_Mats/Top_Colour_Combo.Top_Colour_Combo" :!class /Script/Engine.PrimitiveComponent)) ; Dynamic material to change colour of eyelet when touched
  (Variables|Default|SetColourTopMat _returnvalue)
  (bind _returnvalue_2 (Rendering|Material|CreateDynamicMaterialInstance (Variables|Default|GetColourBottomAurora) 0 "/Game/Materials/Environment_Mats/Bottom_COlour_Combo.Bottom_COlour_Combo" :!class /Script/Engine.PrimitiveComponent)) ; Dynamic material to change colour of eyelet when touched
  (Variables|Default|SetColourBottomMat _returnvalue_2)
  (bind _returnvalue_3 (Rendering|Material|CreateDynamicMaterialInstance (Variables|Default|GetCombinedColourStripe) 0 "/Game/Materials/Environment_Mats/Mid_COlour_Combo.Mid_COlour_Combo" :!class /Script/Engine.PrimitiveComponent)) ; Dynamic material to change colour of eyelet when touched
  (Variables|Default|SetColourMiddleMat _returnvalue_3))