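; Level tile that recycles itself as the VeilCharacter moves through an endless chain of spawned tiles.
; Overlapping its TriggerZone starts a short delay, then, if the character is still alive, asks the TileSpawner for a new tile and destroys this one.
; Cleanup also destroys the Tear and its Eyelets on tear tiles, or the tile's Enemies on other tiles.
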(event OnComponentBeginOverlap(TriggerZone)
  (params (OverlappedComponent :type Primitive%20Component%20Object%20Reference) (OtherActor :type Actor%20Object%20Reference) (OtherComp :type Primitive%20Component%20Object%20Reference) (OtherBodyIndex :type Integer) (bFromSweep :type Boolean) (SweepResult :type Hit%20Result%20Structure%20%28by%20ref%29))
  (bind _mytear (Variables|Default|GetmyTear))
  ;[1 1 1] Check collision, when TriggerZone is ovelapped by VeilCharacter, a new tile is spawn at the spawn point
  (bind _asveil_character (Utilities|Casting|CastToVeilCharacter OtherActor))
  (Utilities|FlowControl|Delay 1.0) ; Delay to not fall and give player time to go to next tile
  (if (not (Variables|/Game/Blueprints/VeilCharacter.VeilCharacter_C|GetisDead _asveil_character))
    (Default|SpawnTileatSpawnPoint (Variables|Default|GetTileSpawner))
    (Actor|DestroyActor) ; Destroy current tile
    (if (Variables|Default|GetisTearTile)
      (for _array_element (Variables|/Game/Blueprints/BaseTear.BaseTear_C|GetEyelets _mytear)
        (Actor|DestroyActor _array_element))
      (Actor|DestroyActor _mytear)
      (else
        ;[1 1 1] Destroying all enemies on that tile to free memory
        (for _array_element_2 (Variables|Default|GetEnemies)
          (Actor|DestroyActor _array_element_2))))))

(event EventBeginPlay)

(event Collision|EventActorBeginOverlap
  (params (OtherActor :type Actor%20Object%20Reference)))

(event EventTick
  (params (DeltaSeconds :type Float%20%28single-precision%29)))

(fn ConstructionScript)